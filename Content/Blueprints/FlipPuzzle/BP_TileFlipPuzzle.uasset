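; Tile flip puzzle actor that builds a clickable grid of static mesh tiles.
; The construction script spawns tile components from Rows, Columns and TileMesh at fixed spacing and stores them in Tiles.
; A left mouse click traces from the cursor on Visibility and passes the hit static mesh component to FlipTiles, whose body is not shown here.
; FlipAdjacentTiles is an empty stub.
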(event `Key|LeftMouseButton`
  (params (Key :type "Key Structure"))
  (:`Pressed`
    (bind _returnvalue (`PuzzleDungeonUtilities.TraceFromMouse` (`GameplayStatics.GetPlayerController` 0) "ECC_Visibility"))
    (bind (_bblockinghit _binitialoverlap _time _distance _location _impactpoint _normal _impactnormal _physmat _hitactor _hitcomponent) (`GameplayStatics.BreakHitResult` _returnvalue))
    (if _bblockinghit
      (bind _asstatic_mesh_component (cast `StaticMeshComponent` _hitcomponent))
      (`self.FlipTiles` _asstatic_mesh_component))))

(fn `FlipAdjacentTiles`
  (params (Index :type Integer)))

(fn `UserConstructionScript`
  (locals (Tile :type "StaticMeshComponent Object Reference"))
  (`KismetArrayLibrary.Array_Clear` (`self.Tiles`))
  (for _index (range (+ (`self.Rows`) 1))
    (for _index_2 (range (+ (`self.Columns`) 1))
      (bind _returnvalue (`AddComponent|NODE_AddStaticMeshComponent-0` :`bManualAttachment` true :`RelativeTransform` (`KismetMathLibrary.MakeTransform` (`KismetMathLibrary.MakeVector` (* _index_2 205.0) (* _index 205.0)))))
      (set `local.Tile` _returnvalue)
      (`StaticMeshComponent.SetStaticMesh` (`local.Tile`) (`self.TileMesh`))
      (`SceneComponent.K2_AttachToComponent` (`local.Tile`) (`self.DefaultSceneRoot`) "None" "KeepRelative" "KeepRelative" "KeepRelative" true)
      (`KismetArrayLibrary.Array_Add` (`self.Tiles`) (`local.Tile`)))))