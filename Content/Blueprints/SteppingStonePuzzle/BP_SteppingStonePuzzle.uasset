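; Stepping stone memory puzzle that briefly shows the player a configured set of tiles to click.
; On BeginPlay it waits, highlights the PuzzleConfig tiles with the AliasMaster material, then restores their default material.
; Left clicks trace from the mouse and pass the hit mesh to OnTileClicked, whose result picks the tile's material.
; Tile lookup and click evaluation are defined outside these graphs; the completion event only prints success and score.
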(event `self.ReceiveBeginPlay`
  (add `self.OnPuzzleComplete` (delegate `PuzzleCompleteEvent`))
  (`KismetSystemLibrary.Delay` 2.0)
  (for _array_element (`self.PuzzleConfig`)
    (bind _returnvalue (`self.GetTile` _array_element))
    (`PrimitiveComponent.SetMaterial` _returnvalue 0 "/DatasmithContent/Materials/AliasMaster.AliasMaster"))
  (`KismetSystemLibrary.Delay` 1.5)
  (for _array_element_2 (`self.PuzzleConfig`)
    (bind _returnvalue_2 (`self.GetTile` _array_element_2))
    (`PrimitiveComponent.SetMaterial` _returnvalue_2 0 "/Engine/EngineMaterials/DefaultMaterial.DefaultMaterial")))

(event `PuzzleCompleteEvent` :!signature `self.OnPuzzleComplete`
  (params (Success :type Boolean) (Score :type "Float (double-precision)"))
  (`KismetSystemLibrary.PrintString` (`KismetStringLibrary.Concat_StrStr` (`KismetStringLibrary.Conv_BoolToString` Success) ", " (`KismetStringLibrary.Conv_DoubleToString` Score))))

(event `Key|LeftMouseButton`
  (params (Key :type "Key Structure"))
  (:`Pressed`
    (bind _returnvalue (`PuzzleDungeonUtilities.TraceFromMouse` (`GameplayStatics.GetPlayerController` 0) "ECC_Visibility"))
    (bind (_bblockinghit _binitialoverlap _time _distance _location _impactpoint _normal _impactnormal _physmat _hitactor _hitcomponent) (`GameplayStatics.BreakHitResult` _returnvalue))
    (if _bblockinghit
      (bind _asstatic_mesh_component (cast `StaticMeshComponent` _hitcomponent))
      (bind _returnvalue_2 (`self.OnTileClicked` _asstatic_mesh_component))
      (if _returnvalue_2
        (`PrimitiveComponent.SetMaterial` _asstatic_mesh_component 0 "/DatasmithContent/Materials/AliasMaster.AliasMaster")
        (else
          (`PrimitiveComponent.SetMaterial` _asstatic_mesh_component 0 "/Engine/EngineMaterials/DefaultMaterial.DefaultMaterial"))))))

(fn `UserConstructionScript`)