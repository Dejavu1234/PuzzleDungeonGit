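; MirrorBase is a clickable mirror for a beam-reflection puzzle that passes a reflecting state to the mirror it faces.
; While reflecting, it line-traces forward on Tick with debug drawing, switching on a mirror hit from the front and remembering it.
; A miss or back-side hit switches that remembered mirror off; hits on other actors leave it unchanged.
; Clicking cycles three rotation entries, adding each yaw to the current rotation.
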(event `self.ReceiveBeginPlay`)

(event `self.ReceiveTick`
  (params (DeltaSeconds :type "Float (single-precision)"))
  (bind _staticmesh (`self.StaticMesh`))
  (bind _mirrorbeinghit (`self.MirrorBeingHit`))
  (bind _returnvalue (`SceneComponent.K2_GetComponentLocation` _staticmesh))
  (if (`self.IsReflecting`)
    (bind (_outhit _returnvalue_2) (`KismetSystemLibrary.LineTraceSingle` :`Start` _returnvalue :`End` (+ _returnvalue (* (`SceneComponent.GetForwardVector` _staticmesh) 2000.0)) :`TraceChannel` "TraceTypeQuery1" :`DrawDebugType` "ForDuration" :`DrawTime` 0.1))
    (if _returnvalue_2
      (bind (_bblockinghit _binitialoverlap _time _distance _location _impactpoint _normal _impactnormal _physmat _hitactor) (`GameplayStatics.BreakHitResult` _outhit))
      (bind _asmirror_base (cast `/Game/Blueprints/MirrorPuzzle/MirrorBase` _hitactor))
      (bind _returnvalue_3 (`PuzzleDungeonUtilities.GetPointIsBehindObject` (`/Game/Blueprints/MirrorPuzzle/MirrorBase.StaticMesh` _asmirror_base) _impactpoint))
      (if _returnvalue_3
        (`/Engine/EditorBlueprintResources/StandardMacros.IsValid` _mirrorbeinghit :!label _label
          (:`Is Valid`
            (set `/Game/Blueprints/MirrorPuzzle/MirrorBase.IsReflecting` false _mirrorbeinghit)))
        (else
          (bind _asmirror_base_2 (cast `/Game/Blueprints/MirrorPuzzle/MirrorBase` _hitactor))
          (set `/Game/Blueprints/MirrorPuzzle/MirrorBase.IsReflecting` true _asmirror_base_2)
          (set `self.MirrorBeingHit` _asmirror_base_2)))
      (else
        (goto _label)))))

(event `self.StaticMesh.OnClicked`
  (params (TouchedComponent :type "PrimitiveComponent Object Reference") (ButtonPressed :type "Key Structure"))
  (bind (_returnvalue_roll _returnvalue_pitch _returnvalue_yaw) (`KismetMathLibrary.BreakRotator` (`SceneComponent.K2_GetComponentRotation` (`self.StaticMesh`))))
  (bind (_output_roll _output_pitch _output_yaw) (`KismetMathLibrary.BreakRotator` (`|GetArrayItem` (`self.ArrayOfRotations`) (`self.CurrentRotation`))))
  (bind _output_get (set `self.CurrentRotation` (+ (`self.CurrentRotation`) 1)))
  (if (> _output_get 2)
    (set `self.CurrentRotation` 0))
  (`SceneComponent.K2_SetWorldRotation` (`self.StaticMesh`) (`KismetMathLibrary.MakeRotator` _returnvalue_roll _returnvalue_pitch (+ _returnvalue_yaw _output_yaw)) false false))

(fn `UserConstructionScript`)